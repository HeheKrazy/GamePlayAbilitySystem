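; GA_MeleeAttack is an enemy gameplay ability for a melee attack.
; It motion-warps the avatar toward its combat target and plays a random tagged attack montage.
; When the montage's tagged event arrives, it gathers live players in a small sphere at the combat socket, damages non-friends and triggers their blood effect.
; A hit fires the melee impact GameplayCue, and the ability ends after the event or when the montage finishes.
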(event Ability|EventActivateAbility
  (bind _returnvalue (Ability|GetAvatarActorfromActorInfo))
  (bind _returnvalue_2 (Ability|GetAvatarActorfromActorInfo))
  (Variables|Default|SetHasHitTarget false)
  (bind _returnvalue_3 (Class|OverlapInterface|GetCombatTarget(Message) _returnvalue))
  (bind _ascombat_interface (Utilities|Casting|CastToCombatInterface _returnvalue))
  (Class|CombatInterface|UpdateWarpMotionFacingTarget _ascombat_interface (Transformation|GetActorLocation _returnvalue_3))
  (bind _returnvalue_4 (Class|CombatInterface|GetAttackMontages(Message) (Ability|GetAvatarActorfromActorInfo)))
  (bind _output_get (Variables|Default|SetTaggedMontage (Class|HKDamageGameplayAbility|GetRandomTaggedMontagefromArray _returnvalue_4)))
  (Variables|Default|SetMontage (.Montage (Utilities|Struct|BreakTaggedMontage _output_get)))
  (Variables|Default|SetMontage%20Tag (.MontageTag (Utilities|Struct|BreakTaggedMontage _output_get)))
  (Variables|Default|SetSocket%20Tag (.SocketTag (Utilities|Struct|BreakTaggedMontage _output_get)))
  (Variables|Default|SetImpact%20Sound (.ImpactSound (Utilities|Struct|BreakTaggedMontage _output_get)))
  (|PlayMontageandWaitProxy "None" (Variables|Default|GetMontage) 1.0 "None" false 1.0 0.0
    (:then
      (Ability|Tasks|WaitGameplayEvent (Variables|Default|GetMontage%20Tag) 0
        (:EventReceived
          (bind _returnvalue_5 (Class|CombatInterface|GetCombatSocketLocation(Message) _returnvalue_2 (Variables|Default|GetSocket%20Tag)))
          (Variables|Default|SetCombatSocketLocation _returnvalue_5)
          (bind _outoverlappingactors (Class|HKAbilitySystemLibrary|GetLivePlayersWithinRadius self (Utilities|Array|MakeArray _returnvalue_2) 45.0 (Variables|Default|GetCombatSocketLocation)))
          (for _array_element _outoverlappingactors
            (if (Class|HKAbilitySystemLibrary|IsNotFriend (Ability|GetAvatarActorfromActorInfo) _array_element)
              (Class|HKDamageGameplayAbility|CauseDamage _array_element)
              (Variables|Default|SetHasHitTarget true)
              (Class|CombatInterface|GetBloodEffect(Message) _array_element)))
          (if (Variables|Default|GetHasHitTarget)
            (bind _returnvalue_6 (Class|OverlapInterface|GetCombatTarget(Message) (Ability|GetAvatarActorfromActorInfo)))
            (Class|GameplayAbility|ExecuteGameplayCuewithParams "(TagName=\"GameplayCue.MeleeImpact\")" (Ability|GameplayCue|MakeGameplayCueParameters :AggregatedSourceTags (GameplayTags|MakeGameplayTagContainerfromTag (Variables|Default|GetMontage%20Tag)) :Location (Variables|Default|GetCombatSocketLocation) :EffectCauser (Ability|GetAvatarActorfromActorInfo) :SourceObject _returnvalue_6)))
          (Ability|EndAbility))))
    (:OnCompleted
      (Ability|EndAbility :!label _label))
    (:OnInterrupted
      (goto _label))
    (:OnCancelled
      (goto _label))))